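; BP_Demon is an enemy that chases the player and raises their Anxiete on contact.
; Every Tick it either issues AIMoveTo toward the player or, while Stuned, waits out a short delay; it starts stunned at BeginPlay.
; Getting within close range stuns the demon and increments the player's Anxiete, with DoOnce gates limiting repeats.
; Reaching AnxieteMax only prints "Dead".
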(event EventTick
  (params (DeltaSeconds :type Float%20%28single-precision%29))
  (bind _playerref (Variables|Default|GetPlayerRef))
  (if (Variables|Default|GetStuned)
    (Utilities|FlowControl|DoOnce false :!label _label
      (:Completed
        (Utilities|FlowControl|Delay 2.0)
        (Variables|Default|SetStuned false)
        (goto _label Reset)))
    (else
      (AI|AIMoveTo self "0, 0, 0" (Game|GetPlayerCharacter 0) 5.0 false
        (:then
          (if (<= (Math|Vector|VectorLength (- (Transformation|GetActorLocation) (Transformation|GetActorLocation (Variables|Default|GetPlayerRef)))) 75.0)
            (Variables|Default|SetStuned true)
            (Utilities|FlowControl|DoOnce false :!label _label_2
              (:Completed
                (Variables|Default|SetStuned true)
                (bind _output_get (Variables|/Game/ThirdPerson/Blueprints/BP_ThirdPersonCharacter.BP_ThirdPersonCharacter_C|SetAnxiete _playerref (+ (Variables|/Game/ThirdPerson/Blueprints/BP_ThirdPersonCharacter.BP_ThirdPersonCharacter_C|GetAnxiete _playerref) 1.0)))
                (if (>= _output_get (Variables|/Game/ThirdPerson/Blueprints/BP_ThirdPersonCharacter.BP_ThirdPersonCharacter_C|GetAnxiete_max _playerref))
                  (Utilities|FlowControl|DoOnce false
                    (:Completed
                      (Development|PrintString "Dead" true true "(R=1.000000,G=0.000000,B=0.028078,A=1.000000)")))
                  (else
                    (Utilities|FlowControl|Delay 2.0)
                    (Variables|Default|SetStuned false)
                    (goto _label_2 Reset)))))))))))

(event EventBeginPlay
  (bind _asbp_third_person_character (Utilities|Casting|CastToBP_ThirdPersonCharacter (Game|GetPlayerCharacter 0)))
  (Variables|Default|SetPlayerRef _asbp_third_person_character)
  (Variables|Default|SetStuned true))

(fn ConstructionScript)